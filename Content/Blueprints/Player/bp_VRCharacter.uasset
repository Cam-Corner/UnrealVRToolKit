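; VR player character that drives a spectator camera and a trailing storage root.
; BeginPlay spawns BP_SpectatorCamera at the VR camera transform, and Tick snaps it to that transform every frame.
; While that camera is valid, Tick also eases StorageRootComp toward CharacterCap's location and rotation.
; The easing is a fixed-alpha lerp without delta time, so its speed depends on frame rate.
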(event `self.ReceiveBeginPlay`
  (bind _returnvalue (`self.GetVRCameraTransorm`))
  (bind _returnvalue_2 (`|SpawnActorFromClass` "/VRToolKit/Blueprints/Player/BP_SpectatorCamera.BP_SpectatorCamera_C" _returnvalue "Undefined" "OverrideRootScale" null null))
  (set `self.SpectatorCamera` _returnvalue_2))

(event `self.ReceiveTick`
  (params (DeltaSeconds :type "Float (single-precision)"))
  (bind __storagerootcomp (`self._StorageRootComp`))
  (bind _spectatorcamera (`self.SpectatorCamera`))
  (bind __charactercap (`self._CharacterCap`))
  (bind _returnvalue (`self.GetVRCameraTransorm`))
  (if (`KismetSystemLibrary.IsValid` _spectatorcamera)
    (`self.K2_SetActorTransform` _spectatorcamera _returnvalue false false)
    (`SceneComponent.K2_SetWorldLocation` __storagerootcomp (`KismetMathLibrary.VLerp` (`SceneComponent.K2_GetComponentLocation` __storagerootcomp) (`SceneComponent.K2_GetComponentLocation` __charactercap) 0.25) false false)
    (`SceneComponent.K2_SetWorldRotation` __storagerootcomp (`KismetMathLibrary.RLerp` (`SceneComponent.K2_GetComponentRotation` __storagerootcomp) (`SceneComponent.K2_GetComponentRotation` __charactercap) 0.25 true) false false)))

(fn `UserConstructionScript`)