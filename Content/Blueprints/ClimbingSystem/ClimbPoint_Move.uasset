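; Moving climb point for the climbing system that travels back and forth between its starting location and an offset set by MoveAmount.
; BeginPlay caches both endpoints, and Tick moves the actor toward the one selected by the MoveUp flag.
; Each frame lerps from the current location, easing into the target, and the flag flips once within a small tolerance.
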(event `self.ReceiveBeginPlay`
  (bind _output_get (set `self.StartLoc` (`self.K2_GetActorLocation`)))
  (set `self.EndLoc` (+ _output_get (`self.MoveAmount`))))

(event `self.ReceiveTick`
  (params (DeltaSeconds :type "Float (single-precision)"))
  (if (`self.MoveUp`)
    (`self.K2_SetActorLocation` (`KismetMathLibrary.VLerp` (`self.K2_GetActorLocation`) (`self.EndLoc`) (* (`self.LerpSpeed`) DeltaSeconds)))
    (if (== (`self.K2_GetActorLocation`) (`self.EndLoc`) :`ErrorTolerance` 2.0)
      (set `self.MoveUp` false))
    (else
      (`self.K2_SetActorLocation` (`KismetMathLibrary.VLerp` (`self.K2_GetActorLocation`) (`self.StartLoc`) (* (`self.LerpSpeed`) DeltaSeconds)))
      (if (== (`self.K2_GetActorLocation`) (`self.StartLoc`) :`ErrorTolerance` 2.0)
        (set `self.MoveUp` true)))))

(fn `UserConstructionScript`)