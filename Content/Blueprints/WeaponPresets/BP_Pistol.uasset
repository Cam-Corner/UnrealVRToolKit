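; Pistol weapon preset Blueprint that wires an auto-loading slider action and a reload system onto the gun.
; BeginPlay links the action to the item mesh, slider grab, hand grab pose and reload system, and also registers the reload system on the gun.
; Tick only reads slider percentage.
; Logic for updating slider, trigger and magazine values and hiding the clip bone is disconnected and never runs.
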(event `self.ReceiveBeginPlay`
  (bind _autoloadingaction (`self.AutoLoadingAction`))
  (bind _reloadsystem (`self.ReloadSystem`))
  (`AutoLoadingAction.SetupComponent` _autoloadingaction self (`self._ItemMesh`))
  (`AutoLoadingAction.SetSliderComp` _autoloadingaction (`self.SliderGrab`))
  (`AutoLoadingAction.SetReloadSystem` _autoloadingaction _reloadsystem)
  (`self.SetReloadSystem` _reloadsystem)
  (`FirearmAction.SetHandGrabPos` (`self.AutoLoadingAction`) (`self.SliderGrabPose`)))

(event `self.ReceiveTick`
  (params (DeltaSeconds :type "Float (single-precision)"))
  (bind _returnvalue (`AutoLoadingAction.GetSliderPercentage` (`self.AutoLoadingAction`))))

(fn `UserConstructionScript`)